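; Player Blueprint for a remote-control handset that drives a robot and triggers its camera.
; WASD sets robot velocity and rotation values plus target thumbstick angles, which Tick eases toward with a rotator lerp while lighting the action lamp during input.
; Space calls TakePicture on BP_Robot, then timelines animate the button and the feed screen's buffering through dynamic materials, with a DoOnce and delay acting as cooldown.
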(event `self.ReceiveBeginPlay`
  (bind _robotcontroller (`self.RobotController`))
  (bind _returnvalue (`PrimitiveComponent.CreateDynamicMaterialInstance` _robotcontroller 3 (`PrimitiveComponent.GetMaterial` _robotcontroller 3) "None"))
  (set `self.DynamicFeedMaterial` _returnvalue)
  (`MaterialInstanceDynamic.SetScalarParameterValue` (`self.DynamicFeedMaterial`) "BufferPercent" 0.0)
  (bind _returnvalue_2 (`PrimitiveComponent.CreateDynamicMaterialInstance` (`self.RobotController`) 2 (`PrimitiveComponent.GetMaterial` _robotcontroller 2) "None"))
  (set `self.ActionLampMaterial` _returnvalue_2))

(event `Key|A`
  (params (Key :type "Key Structure"))
  (:`Pressed`
    (set `self.DesiredRotThumbRot` 50.0)
    (set `self.RobotRotation` 1.0))
  (:`Released`
    (set `self.DesiredRotThumbRot` 0.0 :!label _label)
    (set `self.RobotRotation` 0.0)))

(event `Key|D`
  (params (Key :type "Key Structure"))
  (:`Pressed`
    (set `self.DesiredRotThumbRot` -50.0)
    (set `self.RobotRotation` -1.0))
  (:`Released`
    (goto _label)))

(event `Key|W`
  (params (Key :type "Key Structure"))
  (:`Pressed`
    (set `self.DesiredVelThumbRot` 50.0)
    (set `self.RobotVelocity` 1.0))
  (:`Released`
    (set `self.DesiredVelThumbRot` 0.0 :!label _label_2)
    (set `self.RobotVelocity` 0.0)))

(event `Key|S`
  (params (Key :type "Key Structure"))
  (:`Pressed`
    (set `self.DesiredVelThumbRot` -50.0)
    (set `self.RobotVelocity` -1.0))
  (:`Released`
    (goto _label_2)))

(event `self.ReceiveTick`
  (params (DeltaSeconds :type "Float (single-precision)"))
  (bind _controller_thumbrot (`self.Controller_ThumbRot`))
  (bind _controller_thumbvel (`self.Controller_ThumbVel`))
  (bind (_relativerotation_roll _relativerotation_pitch _relativerotation_yaw) (`KismetMathLibrary.BreakRotator` (`SceneComponent.RelativeRotation` _controller_thumbrot)))
  (bind (_relativerotation_roll_2 _relativerotation_pitch_2 _relativerotation_yaw_2) (`KismetMathLibrary.BreakRotator` (`SceneComponent.RelativeRotation` _controller_thumbvel)))
  (`|ExecutionSequence`
    (:`then_2`
      (`SceneComponent.K2_SetRelativeRotation` _controller_thumbvel (`KismetMathLibrary.RLerp` (`KismetMathLibrary.MakeRotator` _relativerotation_roll_2 _relativerotation_pitch_2 _relativerotation_yaw_2) (`KismetMathLibrary.MakeRotator` (`self.DesiredVelThumbRot`) _relativerotation_pitch_2 _relativerotation_yaw_2) 0.1 true) false false)
      (`SceneComponent.K2_SetRelativeRotation` _controller_thumbrot (`KismetMathLibrary.RLerp` (`KismetMathLibrary.MakeRotator` _relativerotation_roll _relativerotation_pitch _relativerotation_yaw) (`KismetMathLibrary.MakeRotator` _relativerotation_roll _relativerotation_pitch (`self.DesiredRotThumbRot`)) 0.1 true) false false)
      (`MaterialInstanceDynamic.SetScalarParameterValue` (`self.ActionLampMaterial`) "Power" (select `bool` (or (> (`KismetMathLibrary.Abs` (`self.RobotVelocity`)) 0.0) (> (`KismetMathLibrary.Abs` (`self.RobotRotation`)) 0.0) (> (* (stale `Key|SpaceBar` _btn) 10.0) 0.0)) :`false` 0.001 :`true` 1.0 :!type "Float (single-precision)")))))

(event `Key|SpaceBar`
  (params (Key :type "Key Structure"))
  (:`Pressed`
    (`/Engine/EditorBlueprintResources/StandardMacros.DoOnce` false :!label _label_3
      (:`Completed`
        (`MaterialInstanceDynamic.SetScalarParameterValue` (`self.DynamicFeedMaterial`) "BufferPercent" 0.0)
        (bind _returnvalue (`GameplayStatics.GetActorOfClass` "/Game/Blueprints/BP_Robot.BP_Robot_C"))
        (`/Game/Blueprints/BP_Robot.TakePicture` _returnvalue)
        (`|ExecutionSequence`
          (:`then_0`
            (bind (_direction _btn) (`Timeline|TakePictureAnim` :!via `PlayFromStart`)
              (:`Update`
                (bind _returnvalue_2 (* _btn 10.0))
                (`SceneComponent.K2_SetRelativeLocation` (`self.Controller_Button`) (`KismetMathLibrary.MakeVector` _returnvalue_2) false false)
                (`MaterialInstanceDynamic.SetScalarParameterValue` (`self.ActionLampMaterial`) "Power" (`KismetMathLibrary.Conv_BoolToDouble` (> _returnvalue_2 0.0))))))
          (:`then_1`
            (bind (_direction_2 _buffer) (`Timeline|BufferImage` :!via `PlayFromStart`)
              (:`Update`
                (`MaterialInstanceDynamic.SetScalarParameterValue` (`self.DynamicFeedMaterial`) "BufferPercent" _buffer))))
          (:`then_2`
            (`KismetSystemLibrary.Delay` 3.0)
            (goto _label_3 :!via `Reset`)))))))

(fn `UserConstructionScript`)