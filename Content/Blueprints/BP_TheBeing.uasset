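; The Being is a stalker entity that activates after a three-minute delay and hunts BP_Robot, with audio and footstep cues.
; When seen (render check, vision cone, line trace), it freezes, flees to a random navigable point, then increments Stage, which scales its chase speed.
; Reaching the robot attaches it to the entity's jumpscare socket and sets Stage to 999; a further sighting increment triggers the jumpscare sound and quits the game.
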(event `self.ReceiveBeginPlay`
  (bind _returnvalue (`GameplayStatics.GetActorOfClass` "/Game/Blueprints/BP_Robot.BP_Robot_C"))
  (set `self.Robot` _returnvalue)
  (set `self.IsActive` false)
  (`AudioComponent.SetVolumeMultiplier` (`self.Audio`) 0.0)
  (`KismetSystemLibrary.Delay` 180.0)
  (set `self.IsActive` true)
  (`AudioComponent.SetVolumeMultiplier` (`self.Audio`) 5.0))

(event `self.ReceiveTick`
  (params (DeltaSeconds :type "Float (single-precision)"))
  (bind _robot (`self.Robot`))
  (bind _stage (`self.Stage`))
  (bind _stage_2 (`self.Stage`))
  (bind _robot_2 (`self.Robot`))
  (bind _robot_3 (`self.Robot`))
  (bind _returnvalue (`self.K2_GetActorLocation` (`self.Robot`)))
  (if (`self.IsActive`)
    (`|ExecutionSequence`
      (:`then_0`
        (bind (_outhit _returnvalue_2) (`KismetSystemLibrary.LineTraceSingle` (`self.K2_GetActorLocation` _robot_2) (`SceneComponent.K2_GetComponentLocation` (`self.Sphere`)) "TraceTypeQuery1" false (`|MakeArray` _robot_2 self :!type "Actor Object Reference")))
        (if (and (`self.WasRecentlyRendered` 0.05) (`KismetArrayLibrary.Array_Contains` (`PrimitiveComponent.GetOverlappingActors` (`/Game/Blueprints/BP_Robot.VisionCone` (`self.Robot`)) null) self) (not _returnvalue_2))
          (`/Engine/EditorBlueprintResources/StandardMacros.DoOnce` false :!label _label
            (:`Completed`
              (set `CharacterMovementComponent.MaxWalkSpeed` 0.0 (`self.CharacterMovement`))
              (`AudioComponent.SetVolumeMultiplier` (`self.Audio`) 0.0)
              (`KismetSystemLibrary.Delay` (`KismetMathLibrary.RandomFloatInRange` 2.0 5.0))
              (`self.RunAway`)
              (`KismetSystemLibrary.Delay` 5.0)
              (`AudioComponent.SetVolumeMultiplier` (`self.Audio`) 3.0)
              (set `self.FootstepInterval` 1.5)
              (`AudioComponent.SetSound` (`self.Audio`) "/Game/Sounds/EntityNearby.EntityNearby")
              (`/Engine/EditorBlueprintResources/StandardMacros.IncrementInt` (`self.Stage`)
                (:`  `
                  (goto _label :!via `Reset`)))))))
      (:`then_1`
        (if (`self.IsRunning`)
          (`/Engine/EditorBlueprintResources/StandardMacros.DoOnce` false :!label _label_2
            (:`Completed`
              (`GameplayStatics.SpawnSoundAttached` "/Game/Sounds/SND_CUE_CarpetFoostep.SND_CUE_CarpetFoostep" (`self.Mesh`) "None" (0.0 0.0 0.0) (struct) "KeepRelativeOffset" true 5.0 1.0 0.0 "/Game/Sounds/DefaultAttenuation.DefaultAttenuation" null)
              (`KismetSystemLibrary.Delay` (`self.FootstepInterval`))
              (goto _label_2 :!via `Reset`)))))
      (:`then_2`
        (if (and (> _stage 0) (< _stage_2 999))
          (set `CharacterMovementComponent.MaxWalkSpeed` (* _stage 100.0) (`self.CharacterMovement`))
          (`|AIMoveTo` self _returnvalue null 75.0
            (:`OnSuccess`
              (`/Engine/EditorBlueprintResources/StandardMacros.DoOnce` false
                (:`Completed`
                  (`SkeletalMeshComponent.SetAnimationMode` (`self.Mesh`) "AnimationSingleNode")
                  (`SkeletalMeshComponent.SetAnimation` (`self.Mesh`) "/Game/Geometry/TheEntity_Sit.TheEntity_Sit")
                  (`self.K2_SetActorRotation` (`KismetMathLibrary.FindLookAtRotation` (`self.K2_GetActorLocation`) (`self.K2_GetActorLocation` (`self.Robot`))) true)
                  (set `CharacterMovementComponent.MaxWalkSpeed` 0.0 (`self.CharacterMovement`))
                  (set `/Game/Blueprints/BP_Robot.Speed` 0.0 _robot)
                  (set `/Game/Blueprints/BP_Robot.RotSpeed` 0.0 _robot)
                  (`GameplayStatics.PlaySoundAtLocation` "/Game/Sounds/RobotPickUp.RobotPickUp" (`self.K2_GetActorLocation` _robot) (struct) 5.0 1.0 0.0 "/Game/Sounds/DefaultAttenuation.DefaultAttenuation" null null)
                  (set `self.Stage` 999)
                  (`PrimitiveComponent.SetSimulatePhysics` (`/Game/Blueprints/BP_Robot.Body` _robot_3) false)
                  (`self.K2_AttachToComponent` _robot_3 (`self.Mesh`) "JumpscarePoint" "SnapToTarget" "SnapToTarget" "KeepWorld" false)
                  (`self.K2_SetActorRelativeRotation` (`self.Robot`) (struct :`Pitch` 45.0 :`Yaw` -270.0 :`Roll` 80.0) false false)))))
          (elif (== _stage_2 1000)
            (`/Engine/EditorBlueprintResources/StandardMacros.DoOnce` false
              (:`Completed`
                (`GameplayStatics.PlaySoundAtLocation` "/Game/Sounds/EntityJumpscare.EntityJumpscare" _returnvalue (struct) 8.0 1.0 0.0 null null null)
                (`KismetSystemLibrary.Delay` 8.5)
                (`KismetSystemLibrary.QuitGame` null "Quit")))))))))

(event `RunAway`
  (if (< (`self.Stage`) 999)
    (set `CharacterMovementComponent.MaxWalkSpeed` 1000.0 (`self.CharacterMovement`))
    (`|AIMoveTo` self (`NavigationSystemV1.K2_GetRandomLocationInNavigableRadius` (`self.K2_GetActorLocation`) 10000.0 null null) null
      (:`then`
        (set `self.IsRunning` true)
        (set `self.FootstepInterval` 0.3)))))

(fn `UserConstructionScript`)