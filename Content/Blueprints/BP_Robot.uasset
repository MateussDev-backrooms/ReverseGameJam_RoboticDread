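; BP_Robot is a physics-driven robot steered by values read from BP_Player, acting as a remote camera and ear.
; BeginPlay moves the audio listener onto its scene capture component and takes an initial capture.
; Tick pushes and yaws the body from the player's inputs, modulating motor sound volume and pitch.
; TakePicture captures a still with a two-second DoOnce cooldown and ready cue; hard horizontal hits play collision sounds.
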(event `self.ReceiveBeginPlay`
  (bind _returnvalue (`GameplayStatics.GetPlayerController` 0))
  (bind _scenecapturecomponent2d (`self.SceneCaptureComponent2D`))
  (bind _asbp_player (cast `/Game/Blueprints/BP_Player` (`GameplayStatics.GetPlayerCharacter` 0)))
  (set `self.Player` _asbp_player)
  (`PlayerController.SetAudioListenerAttenuationOverride` _returnvalue _scenecapturecomponent2d (0.0 0.0 0.0))
  (`PlayerController.SetAudioListenerOverride` :`self` _returnvalue :`AttachToComponent` _scenecapturecomponent2d)
  (`SceneCaptureComponent2D.CaptureScene` (`self.SceneCaptureComponent2D`)))

(event `self.ReceiveTick`
  (params (DeltaSeconds :type "Float (single-precision)"))
  (bind _player (`self.Player`))
  (bind _body (`self.Body`))
  (bind _scenecapturecomponent2d (`self.SceneCaptureComponent2D`))
  (bind _robotvelocity (`/Game/Blueprints/BP_Player.RobotVelocity` _player))
  (bind _robotrotation (`/Game/Blueprints/BP_Player.RobotRotation` _player))
  (`PrimitiveComponent.AddForce` _body (+ (* (`SceneComponent.GetForwardVector` _scenecapturecomponent2d) (* _robotvelocity (`self.Speed`))) (* (`SceneComponent.GetUpVector` _scenecapturecomponent2d) 100.0)) "None" false)
  (`SceneComponent.K2_AddWorldRotation` _body (`KismetMathLibrary.MakeRotator` 0.0 0.0 (* _robotrotation (`self.RotSpeed`))) false false)
  (`AudioComponent.SetVolumeMultiplier` (`self.RobotMovement`) (`KismetMathLibrary.Conv_BoolToDouble` (> (`KismetMathLibrary.Abs` _robotvelocity) 0.0)))
  (`AudioComponent.SetVolumeMultiplier` (`self.RobotRotation`) (`KismetMathLibrary.Conv_BoolToDouble` (> (`KismetMathLibrary.Abs` _robotrotation) 0.0)))
  (`AudioComponent.SetPitchMultiplier` (`self.RobotMovement`) (`KismetMathLibrary.Lerp` 1.5 1.0 (`KismetMathLibrary.Conv_BoolToDouble` (> (`KismetMathLibrary.VSize` (`self.GetVelocity`)) 5.0)))))

(event `TakePicture`
  (`/Engine/EditorBlueprintResources/StandardMacros.DoOnce` false :!label _label
    (:`Completed`
      (`SceneCaptureComponent2D.CaptureScene` (`self.SceneCaptureComponent2D`))
      (`GameplayStatics.PlaySoundAtLocation` "/Game/Sounds/RobotCamSnap.RobotCamSnap" (`self.K2_GetActorLocation`) (struct) 1.0 1.0 0.0 "/Game/Sounds/DefaultAttenuation.DefaultAttenuation" null null)
      (`KismetSystemLibrary.Delay` 2.0)
      (`GameplayStatics.PlaySound2D` "/Game/Sounds/CamReadyCue.CamReadyCue" 1.0 1.0 0.0 null null)
      (goto _label :!via `Reset`))))

(event `self.ReceiveHit`
  (params (MyComp :type "PrimitiveComponent Object Reference") (Other :type "Actor Object Reference") (OtherComp :type "PrimitiveComponent Object Reference") (bSelfMoved :type Boolean) (HitLocation :type "Vector Structure") (HitNormal :type "Vector Structure") (NormalImpulse :type "Vector Structure") (Hit :type "HitResult Structure (by ref)"))
  (if (> (`KismetMathLibrary.VSize` (`KismetMathLibrary.MakeVector` (.x NormalImpulse) (.y NormalImpulse))) 100.0)
    (`GameplayStatics.PlaySoundAtLocation` "/Game/Sounds/RobotCollision.RobotCollision" HitLocation (struct) 1.0 1.0 0.0 "/Game/Sounds/DefaultAttenuation.DefaultAttenuation" null null)))

(fn `UserConstructionScript`)